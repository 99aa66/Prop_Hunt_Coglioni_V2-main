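; Game state for a multiplayer prop hunt match, tracking hunters and prop hiders and deciding the winning team.
; RepNotify countdowns chain game start, hunter release and match time, each re-arming a one-second delayed decrement on the server and updating countdown text.
; Game start picks a hunter from shuffled players and spawns hiders.
; An empty team or expired match timer sets the winner, triggering GameEnded and its end-of-match sound and animation.
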(event `Countdown_GameStart`
  (`KismetSystemLibrary.Delay` 1.0)
  (bind _result (`/Engine/EditorBlueprintResources/StandardMacros.DecrementInt` (`self.GameStart_Countdown`))
    (:`  `
      (set `self.GameStart_Countdown` _result))))

(event `Countdown_HunterRelease`
  (`KismetSystemLibrary.Delay` 1.0)
  (bind _result (`/Engine/EditorBlueprintResources/StandardMacros.DecrementInt` (`self.HunterRelease_Countdown`))
    (:`  `
      (set `self.HunterRelease_Countdown` _result))))

(event `Countdown_MatchTime`
  (`KismetSystemLibrary.Delay` 1.0)
  (bind _result (`/Engine/EditorBlueprintResources/StandardMacros.DecrementInt` (`self.MatchTime_Countdown`))
    (:`  `
      (set `self.MatchTime_Countdown` _result))))

(fn `Add_Hunter`
  (params (Player :type "PlayerState Object Reference (by ref)"))
  (bind _activehunters (`self.ActiveHunters`))
  (`KismetArrayLibrary.Array_Add` _activehunters Player)
  (set `self.ActiveHunters` _activehunters)
  (`self.Remove_AnActiveProp` Player))

(fn `Check_GameFinished`
  ;[0.05098 0.05098 0.05098] Check if we still have hunters
  (if (<= (`KismetArrayLibrary.Array_Length` (`self.ActiveHunters`)) 0)
    ;[0.05098 0.05098 0.05098] If 0 Hunters are left, the Prop Hiders win
    (set `self.WinnigTeam` "Prop Hiders")
    (else
      ;[0.05098 0.05098 0.05098] Check if we still have prop hiders
      (if (<= (`KismetArrayLibrary.Array_Length` (`self.ActiveProps`)) 0)
        ;[0.05098 0.05098 0.05098] If 0 active props are left, the hunters win
        (set `self.WinnigTeam` "Hunter")))))

(fn `Check_RequiredPlayerAmount`
  (bind _playerarray (`self.PlayerArray`))
  (if (!= (`self.GameStart_Countdown`) 0)
    (`KismetArrayLibrary.Array_Shuffle` _playerarray)
    (set `self.ActiveProps` _playerarray)
    (`self.Set Countdown Text` "Waiting for 1 more player")
    (if (>= (`KismetArrayLibrary.Array_Length` (`self.ActiveProps`)) 2)
      (`self.Countdown_GameStart`))))

(fn `OnRep_GameEnded?`
  (`GameplayStatics.PlaySound2D` "/Game/Sound/success-fanfare-trumpets-6185.success-fanfare-trumpets-6185" 1.0 1.0 0.0 null null)
  (bind _asbp_pc_gameplay (cast `/Game/Blueprint/BP_PC_Gameplay` (`GameplayStatics.GetPlayerController` 0)))
  (`/Game/Blueprint/BP_PC_Gameplay.OC_Play_MatchOver_Animation` _asbp_pc_gameplay))

(fn `OnRep_GameStart_Countdown`
  (`/Engine/EditorBlueprintResources/ActorMacros.Switch Has Authority`
    (:`Authority`
      ;[0.05098 0.05098 0.05098] Set countdown text in UI
      (`self.Set Countdown Text` "Game starts in:" (`KismetStringLibrary.Conv_IntToString` (`self.GameStart_Countdown`)))
      ;[0.05098 0.05098 0.05098] At zero seconds we Start the Game, otherwise continue the countdown
      (if (== (`self.GameStart_Countdown`) 0)
        (`self.StartGame`)
        (else
          (`self.Countdown_GameStart`))))))

(fn `OnRep_HunterRelease_Countdown`
  ;[0.05098 0.05098 0.05098] Play 'Hunters Are Released' sound
  (if (<= (`self.HunterRelease_Countdown`) 0)
    (`GameplayStatics.PlaySound2D` null 1.0 1.0 0.0 null null))
  (`/Engine/EditorBlueprintResources/ActorMacros.Switch Has Authority`
    (:`Authority`
      (`self.Set Countdown Text` "Time till hunter release:" (`KismetStringLibrary.Conv_IntToString` (`self.HunterRelease_Countdown`)))
      (if (<= (`self.HunterRelease_Countdown`) 0)
        (set `self.MatchTime_Countdown` (`self.Initial_MatchTime_Countdown`))
        (bind _returnvalue (`GameplayStatics.GetActorOfClass` "/Game/PropHunt/Blueprints/Core/Gameplay/Actors/BP_HunterDoor.BP_HunterDoor_C"))
        (`/Game/PropHunt/Blueprints/Core/Gameplay/Actors/BP_HunterDoor.SR_OpenDoor` _returnvalue)
        (else
          (`self.Countdown_HunterRelease`))))))

(fn `OnRep_MatchTime_Countdown`
  (`/Engine/EditorBlueprintResources/ActorMacros.Switch Has Authority`
    (:`Authority`
      ;[0.05098 0.05098 0.05098] Set match time countdown in UI
      (`self.Set Countdown Text` "Match time left:" (`KismetStringLibrary.Conv_IntToString` (`self.MatchTime_Countdown`)))
      (if (not (`self.GameEnded?`))
        (if (<= (`self.MatchTime_Countdown`) 0)
          ;[0.05098 0.05098 0.05098] If the match countdown reaches 0, then the Prop Hiders automatically win
          (set `self.WinnigTeam` "Prop Hiders")
          (else
            ;[0.05098 0.05098 0.05098] Otherwise just keep counting down
            (`self.Countdown_MatchTime`)))))))

(fn `OnRep_WinnigTeam`
  (`/Engine/EditorBlueprintResources/ActorMacros.Switch Has Authority`
    (:`Authority`
      (set `self.GameEnded?` true))))

(fn `Remove_AnActiveHunter`
  (params (AciveHunterToRemove :type "PlayerState Object Reference (by ref)"))
  (bind _activehunters (`self.ActiveHunters`))
  (if (not (`self.GameEnded?`))
    (`KismetArrayLibrary.Array_RemoveItem` _activehunters AciveHunterToRemove)
    (set `self.ActiveHunters` _activehunters)
    (`self.Check_GameFinished`)))

(fn `Remove_AnActiveProp`
  (params (ActivePropToRemove :type "PlayerState Object Reference"))
  (bind _activeprops (`self.ActiveProps`))
  (if (not (`self.GameEnded?`))
    (`KismetArrayLibrary.Array_RemoveItem` _activeprops ActivePropToRemove)
    (set `self.ActiveProps` _activeprops)
    (`self.Check_GameFinished`)))

(fn `Set Countdown Text`
  (params (CountdownDescription_Text :type String) (Countdown_Amount :type String))
  (set `self.CountdownDescription_Text` CountdownDescription_Text)
  (set `self.Countdown_Amount` Countdown_Amount))

(fn `Signal_PlayerLeft`
  (params (Player :type "PlayerState Object Reference"))
  (bind _asbp_ps_gameplay (cast `/Game/Blueprint/BP_PS_Gameplay` Player))
  (if (`/Game/Blueprint/BP_PS_Gameplay.IsHunter?` _asbp_ps_gameplay)
    (`self.Remove_AnActiveHunter` _asbp_ps_gameplay)
    (else
      (`self.Remove_AnActiveProp` _asbp_ps_gameplay))))

(fn `StartGame`
  (`/Engine/EditorBlueprintResources/ActorMacros.Switch Has Authority`
    (:`Authority`
      ;[0.05098 0.05098 0.05098] Select the first hunter
      (bind _asbp_ps_gameplay (cast `/Game/Blueprint/BP_PS_Gameplay` (`|GetArrayItem` (`self.ActiveProps`))))
      (set `/Game/Blueprint/BP_PS_Gameplay.IsHunter?` true _asbp_ps_gameplay)
      ;[0.05098 0.05098 0.05098] Spawn all the hiders
      (bind _asbp_gm_gameplay (cast `/Game/Blueprint/BP_GM_Gameplay` (`GameplayStatics.GetGameMode`)))
      (`/Game/Blueprint/BP_GM_Gameplay.Spawn_AllHiders` _asbp_gm_gameplay)
      ;[0.05098 0.05098 0.05098] Start the Hunter Release countdown
      (set `self.HunterRelease_Countdown` (`self.Initial_Ping_Countdown`))
      (`KismetSystemLibrary.PrintString` "spawn characters"))))

(fn `UserConstructionScript`)