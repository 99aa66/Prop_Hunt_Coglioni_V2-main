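; Gameplay game mode for a hide-and-seek match, spawning players as hiders, FPS hunters or spectators.
; It tracks controllers, has GS_Game check the player count on login, and signals it when playing players leave.
; Spawn functions destroy the current pawn, then possess a new one, usually at a random tagged PlayerStart.
; SpawnAllHiders spawns the game state's ActiveProps as hiders, and TravelToLevel issues ServerTravel.
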(event `self.K2_PostLogin`
  (params (NewPlayer :type "PlayerController Object Reference"))
  ;[0.05098 0.05098 0.05098] Player Connection and disconnection
  (`KismetArrayLibrary.Array_Add` (`self.All_PlayerControllers`) NewPlayer)
  ;;[0.05098 0.05098 0.05098] Fire a check to see if we can start the game
  (bind _asgs_game (cast `/Game/Blueprint/GS_Game` (`GameplayStatics.GetGameState`)))
  (`/Game/Blueprint/GS_Game.Check_RequiredPlayerAmount` _asgs_game))

(event `self.K2_OnSwapPlayerControllers`
  (params (OldPC :type "PlayerController Object Reference") (NewPC :type "PlayerController Object Reference"))
  ;[0.05098 0.05098 0.05098] Player Connection and disconnection
  (`KismetArrayLibrary.Array_Add` (`self.All_PlayerControllers`) NewPC))

(event `self.K2_OnLogout`
  (params (ExitingController :type "Controller Object Reference"))
  ;[0.05098 0.05098 0.05098] Player Connection and disconnection
  (bind _asbp_pc_gameplay (cast `/Game/Blueprint/BP_PC_Gameplay` ExitingController))
  (`KismetArrayLibrary.Array_RemoveItem` (`self.All_PlayerControllers`) _asbp_pc_gameplay)
  (if (`/Game/Blueprint/BP_PC_Gameplay.IsPlayingPlayer?` _asbp_pc_gameplay)
    (bind _asgs_game (cast `/Game/Blueprint/GS_Game` (`GameplayStatics.GetGameState`)))
    (`/Game/Blueprint/GS_Game.Signal_PlayerLeft` _asgs_game (`Controller.PlayerState` _asbp_pc_gameplay))))

(fn `Destroy_ControlledPawn`
  (params (Player :type "Controller Object Reference"))
  (bind _returnvalue (`Controller.K2_GetPawn` Player))
  (`/Engine/EditorBlueprintResources/StandardMacros.IsValid` _returnvalue
    (:`Is Valid`
      (`self.K2_DestroyActor` _returnvalue))
    (:`Is Not Valid`
      _))
  (return))

(fn `Get_PlayerStart_WithTag`
  (params (PlayerStart_Tag :type Name))
  (returns (Transform :type "Transform Structure (by ref)"))
  (locals (PlayerStarts :type "Array of PlayerStart Object Reference"))
  (bind _playerstarts (`local.PlayerStarts`))
  (bind _outactors (`GameplayStatics.GetAllActorsOfClassWithTag` "/Script/Engine.PlayerStart" PlayerStart_Tag))
  (set `local.PlayerStarts` _outactors)
  (`KismetArrayLibrary.Array_Shuffle` _playerstarts)
  (bind _output_get (set `local.PlayerStarts` _playerstarts))
  (return (`self.GetTransform` (`|GetArrayItem` _output_get))))

(fn `Spawn Character Hunter`
  (params (Player :type "PlayerController Object Reference") (PlayerStart_Tag :type Name))
  (locals (Spawn_Transform :type "Transform Structure"))
  (`self.Destroy_ControlledPawn` Player)
  (bind _transform (`self.Get_PlayerStart_WithTag` "Hunter"))
  (bind _returnvalue (`|SpawnActorFromClass` "/Game/Player/C_PlayerFPS.C_PlayerFPS_C" _transform "Undefined" "MultiplyWithRoot" (`local.Player`) null))
  (`Controller.Possess` (`local.Player`) _returnvalue))

(fn `Spawn_AllHiders`
  (bind _asgs_game (cast `/Game/Blueprint/GS_Game` (`GameplayStatics.GetGameState`)))
  (for _array_element (`/Game/Blueprint/GS_Game.ActiveProps` _asgs_game)
    (bind _asbp_ps_gameplay (cast `/Game/Blueprint/BP_PS_Gameplay` _array_element))
    (`self.Spawn_Character_Hider` (`PlayerState.GetPlayerController` _asbp_ps_gameplay) "Hider")
    (`KismetSystemLibrary.PrintString` "Spawn Hider")))

(fn `Spawn_Character`
  (params (Player :type "PlayerController Object Reference") (PlayerStart_Tag :type Name))
  (locals (Spawn_Transform :type "Transform Structure"))
  (`self.Destroy_ControlledPawn` Player)
  (bind _transform (`self.Get_PlayerStart_WithTag` PlayerStart_Tag))
  (bind _returnvalue (`|SpawnActorFromClass` "/Game/Player/C_Player.C_Player_C" _transform "Undefined" "MultiplyWithRoot" (`local.Player`) null))
  (`Controller.Possess` (`local.Player`) _returnvalue)
  (`KismetSystemLibrary.PrintText` "Poses"))

(fn `Spawn_Character_Hider`
  (params (Player :type "PlayerController Object Reference") (PlayerStart_Tag :type Name))
  (locals (Spawn_Transform :type "Transform Structure"))
  (`self.Destroy_ControlledPawn` Player)
  (bind _transform (`self.Get_PlayerStart_WithTag` PlayerStart_Tag))
  (bind _returnvalue (`|SpawnActorFromClass` "/Game/Player/C_Player.C_Player_C" _transform "Undefined" "MultiplyWithRoot" (`local.Player`) null))
  (`Controller.Possess` (`local.Player`) _returnvalue))

(fn `Spawn_SpectatePawn`
  (params (Player :type "PlayerController Object Reference") (`SpawnAtPlayerLocation?` :type Boolean) (PlayerTransform :type "Transform Structure"))
  (`self.Destroy_ControlledPawn` Player)
  (if `SpawnAtPlayerLocation?`
    (bind _returnvalue (`|SpawnActorFromClass` "/Game/Blueprint/BP_SpectatingPawn.BP_SpectatingPawn_C" PlayerTransform "Undefined" "MultiplyWithRoot" (`local.Player`) null))
    (`Controller.Possess` (`local.Player`) _returnvalue)
    (else
      (bind _transform (`self.Get_PlayerStart_WithTag` "Start"))
      (bind _returnvalue_2 (`|SpawnActorFromClass` "/Game/Blueprint/BP_SpectatingPawn.BP_SpectatingPawn_C" _transform "Undefined" "MultiplyWithRoot" (`local.Player`) null))
      (`Controller.Possess` (`local.Player`) _returnvalue_2))))

(fn `TravelToLevel`
  (bind _returnvalue (`GameplayStatics.GetCurrentLevelName` true))
  (switch `string` _returnvalue
    (:`Level_1`
      (`KismetSystemLibrary.ExecuteConsoleCommand` "ServerTravel Level_1" null)
      (`KismetSystemLibrary.PrintString` "switch to Level 1"))))

(fn `UserConstructionScript`)